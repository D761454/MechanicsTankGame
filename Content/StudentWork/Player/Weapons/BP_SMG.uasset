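; BP_SMG is a rapid-fire tank weapon that, when triggered, fires projectiles in a random spread cone from the tank's direction arrow.
; A shot counter swaps in a homing projectile after every five SMG rounds and points it at that projectile's own target.
; Completed shots shake the camera and start a short timer cooldown.
; A homing shot without a valid target still spawns, but skips the counter reset, shake and cooldown.
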(event `self.Triggered`
  (bind _directionarrow (`/Game/Blueprints/BP_PlayerCharacter.DirectionArrow` (`self.MyTank`)))
  (bind _returnvalue (`SceneComponent.K2_GetComponentLocation` _directionarrow))
  (bind _returnvalue_2 (`KismetMathLibrary.Conv_VectorToRotator` (`KismetMathLibrary.RandomUnitVectorInConeInDegrees` (`KismetMathLibrary.Conv_RotatorToVector` (`SceneComponent.K2_GetComponentRotation` _directionarrow)) 15.0)))
  (if (not (`self.Cooldown`))
    (if (> (`self.Shots`) 4)
      (bind _returnvalue_3 (`|SpawnActorFromClass` "/Game/StudentWork/Player/Projectiles/BP_Homing_Projectile.BP_Homing_Projectile_C" (`KismetMathLibrary.MakeTransform` _returnvalue _returnvalue_2) "Undefined" "MultiplyWithRoot" null null))
      (bind _my_target (`/Game/StudentWork/Player/Projectiles/BP_Homing_Projectile.My Target` _returnvalue_3))
      (`/Engine/EditorBlueprintResources/StandardMacros.IsValid` _my_target
        (:`Is Valid`
          (set `ProjectileMovementComponent.HomingTargetComponent` (`Actor.RootComponent` _my_target) (`/Game/StudentWork/Player/Projectiles/BP_Homing_Projectile.ProjectileMovement` _returnvalue_3))
          (set `self.Shots` 0)))
      (else
        (`|SpawnActorFromClass` "/Game/StudentWork/Player/Projectiles/BP_SMG_Projectile.BP_SMG_Projectile_C" (`KismetMathLibrary.MakeTransform` _returnvalue _returnvalue_2) "Undefined" "MultiplyWithRoot" null null)
        (set `self.Shots` (+ (`self.Shots`) 1))))
    (`PlayerCameraManager.StartCameraShake` :`self` (`GameplayStatics.GetPlayerCameraManager` 0) :`ShakeClass` "/Game/StudentWork/CamShakes/CS_RegFire.CS_RegFire_C")
    (set `self.Cooldown` true)
    (`KismetSystemLibrary.K2_SetTimerDelegate` (delegate `End Cooldown`) 0.1)))

(event `End Cooldown`
  (set `self.Cooldown` false))

(fn `UserConstructionScript`
  (`parent.UserConstructionScript`))