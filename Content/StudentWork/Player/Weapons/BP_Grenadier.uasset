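; BP_Grenadier is a tank weapon with two fire modes, a lobbed grenade as primary and a missile as secondary.
; Both spawn from the owning tank's DirectionArrow, with the grenade's pitch raised steeply for an arcing launch.
; Each shot plays a projectile sound and a camera shake on the first player's camera.
; Each mode has its own cooldown flag, cleared by a timer, with the missile's lasting longer.
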(event `self.TriggeredSEC`
  (bind _directionarrow (`/Game/Blueprints/BP_PlayerCharacter.DirectionArrow` (`self.MyTank`)))
  ;[1 1 1] Sec fire
  (if (not (`self.Cooldown2`))
    (bind _returnvalue (`|SpawnActorFromClass` "/Game/StudentWork/Player/Projectiles/BP_Missile.BP_Missile_C" (`KismetMathLibrary.MakeTransform` (`SceneComponent.K2_GetComponentLocation` _directionarrow) (`SceneComponent.K2_GetComponentRotation` _directionarrow)) "Undefined" "MultiplyWithRoot" null null))
    (`GameplayStatics.PlaySoundAtLocation` "/Game/StudentWork/Audio_Project_Files/ProjectileMETASOUND.ProjectileMETASOUND" (`self.K2_GetActorLocation`) (struct) 1.0 1.0 0.0 null "/Game/StudentWork/Audio_Project_Files/ProjectileExplosion_SC.ProjectileExplosion_SC" _returnvalue null)
    (`PlayerCameraManager.StartCameraShake` :`self` (`GameplayStatics.GetPlayerCameraManager` 0) :`ShakeClass` "/Game/StudentWork/CamShakes/CS_Death.CS_Death_C")
    (set `self.Cooldown2` true)
    (`KismetSystemLibrary.K2_SetTimerDelegate` (delegate `End Cooldown2`) 3.0)))

(event `End Cooldown2`
  ;[1 1 1] Sec fire
  (set `self.Cooldown2` false))

(event `self.Triggered`
  (bind _directionarrow (`/Game/Blueprints/BP_PlayerCharacter.DirectionArrow` (`self.MyTank`)))
  (bind (_returnvalue_roll _returnvalue_pitch _returnvalue_yaw) (`KismetMathLibrary.BreakRotator` (`SceneComponent.K2_GetComponentRotation` _directionarrow)))
  ;[1 1 1] Primary fire
  (if (not (`self.Cooldown`))
    (bind _returnvalue (`|SpawnActorFromClass` "/Game/StudentWork/Player/Projectiles/BP_Grenade.BP_Grenade_C" (`KismetMathLibrary.MakeTransform` (`SceneComponent.K2_GetComponentLocation` _directionarrow) (`KismetMathLibrary.MakeRotator` _returnvalue_roll (+ _returnvalue_pitch 75.0) _returnvalue_yaw)) "Undefined" "MultiplyWithRoot" null null))
    (`GameplayStatics.PlaySoundAtLocation` "/Game/StudentWork/Audio_Project_Files/ProjectileMETASOUND.ProjectileMETASOUND" (`self.K2_GetActorLocation`) (struct) 1.0 1.0 0.0 null "/Game/StudentWork/Audio_Project_Files/ProjectileExplosion_SC.ProjectileExplosion_SC" _returnvalue null)
    (`PlayerCameraManager.StartCameraShake` :`self` (`GameplayStatics.GetPlayerCameraManager` 0) :`ShakeClass` "/Game/StudentWork/CamShakes/CS_RegFire.CS_RegFire_C")
    (set `self.Cooldown` true)
    (`KismetSystemLibrary.K2_SetTimerDelegate` (delegate `End Cooldown`) 2.0)))

(event `End Cooldown`
  ;[1 1 1] Primary fire
  (set `self.Cooldown` false))

(fn `UserConstructionScript`
  (`parent.UserConstructionScript`))