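; BP_Grenade is a player projectile that explodes on impact.
; When its sphere mesh registers a hit, it applies full radial damage around the mesh and calls a custom event that destroys the actor.
; The same hit chain then plays a distance-scaled explosion camera shake and spawns the explosion Niagara effect at the actor's location, both sequenced after the destroy call.
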(event `DestroyEvent`
  (`self.K2_DestroyActor`))

(event `self.SM_Sphere.OnComponentHit`
  (params (HitComponent :type "PrimitiveComponent Object Reference") (OtherActor :type "Actor Object Reference") (OtherComp :type "PrimitiveComponent Object Reference") (NormalImpulse :type "Vector Structure") (Hit :type "HitResult Structure (by ref)"))
  (`GameplayStatics.ApplyRadialDamage` :`BaseDamage` 50.0 :`Origin` (`SceneComponent.K2_GetComponentLocation` (`self.SM_Sphere`)) :`DamageRadius` 150.0 :`DamageCauser` self :`InstigatedByController` null :`bDoFullDamage` true)
  (`self.DestroyEvent`)
  (`GameplayStatics.PlayWorldCameraShake` "/Game/StudentWork/CamShakes/CS_Explosion.CS_Explosion_C" (`self.K2_GetActorLocation`) 0.1 3000.0 0.1)
  (`NiagaraFunctionLibrary.SpawnSystemAtLocation` "/Game/StudentWork/Particles/Death/NS_Explosion.NS_Explosion" (`self.K2_GetActorLocation`)))

(fn `UserConstructionScript`)