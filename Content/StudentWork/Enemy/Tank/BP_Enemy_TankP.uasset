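; BP_Enemy_TankP is a tank enemy that pursues a target and fires projectiles.
; Tick calls HullToFace every frame, whose logic is defined outside this graph.
; The Move event sends the pawn toward MyTarget with AI MoveTo when that target is valid.
; The Attack event spawns a BP_Tank_Projectile at the FireArrow component's world location and rotation.
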(event `self.ReceiveTick`
  (params (DeltaSeconds :type "Float (single-precision)"))
  (`self.HullToFace`))

(event `self.Move`
  (bind _mytarget (`self.MyTarget`))
  ;[1 1 1] Movement
  (`/Engine/EditorBlueprintResources/StandardMacros.IsValid` _mytarget
    (:`Is Valid`
      (`|AIMoveTo` self (0.0 0.0 0.0) _mytarget 10.0))))

(event `self.Attack`
  (bind _firearrow (`self.FireArrow`))
  ;[1 1 1] Attack
  (`|SpawnActorFromClass` "/Game/StudentWork/Enemy/Tank/BP_Tank_Projectile.BP_Tank_Projectile_C" (`KismetMathLibrary.MakeTransform` (`SceneComponent.K2_GetComponentLocation` _firearrow) (`SceneComponent.K2_GetComponentRotation` _firearrow)) "Undefined" "MultiplyWithRoot" null null))

(fn `UserConstructionScript`
  (`parent.UserConstructionScript`))