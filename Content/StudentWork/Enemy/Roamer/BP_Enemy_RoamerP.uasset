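; BP_Enemy_RoamerP is a roaming enemy that fires projectiles.
; Its Move event sends it by AI move to a random reachable point within a radius of its current location.
; Its Attack event spawns a BP_EnemyProjectile at the position and rotation of its FireArrow component.
; Neither event is called within this file, and construction only runs the parent script.
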(event `self.Move`
  ;[1 1 1] Movement
  (`|AIMoveTo` self (`NavigationSystemV1.K2_GetRandomReachablePointInRadius` (`self.K2_GetActorLocation`) 600.0 null null) null 10.0))

(event `self.Attack`
  (bind _firearrow (`self.FireArrow`))
  ;[1 1 1] Attack
  (`|SpawnActorFromClass` "/Game/StudentWork/Enemy/BP_EnemyProjectile.BP_EnemyProjectile_C" (`KismetMathLibrary.MakeTransform` (`SceneComponent.K2_GetComponentLocation` _firearrow) (`SceneComponent.K2_GetComponentRotation` _firearrow)) "Undefined" "MultiplyWithRoot" null null))

(fn `UserConstructionScript`
  (`parent.UserConstructionScript`))