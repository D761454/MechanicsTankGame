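; Elite Roamer enemy variant that fires elite projectiles at its target.
; Its Attack event checks that the target is valid, then spawns the projectile at the fire arrow, rotated toward the target's location.
; It then plays a MetaSound at the enemy's location with attenuation and concurrency settings, owned by the new projectile.
; The construction script only calls the parent's.
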(event `self.Attack`
  (bind _mytarget (`self.MyTarget`))
  (bind _returnvalue (`SceneComponent.K2_GetComponentLocation` (`self.FireArrow`)))
  ;[1 0 0] Attack Player
  (`/Engine/EditorBlueprintResources/StandardMacros.IsValid` _mytarget
    (:`Is Valid`
      (bind _returnvalue_2 (`|SpawnActorFromClass` "/Game/StudentWork/Enemy/BP_EnemyProjectile_Elite.BP_EnemyProjectile_Elite_C" (`KismetMathLibrary.MakeTransform` _returnvalue (`KismetMathLibrary.FindLookAtRotation` _returnvalue (`self.K2_GetActorLocation` _mytarget))) "Undefined" "MultiplyWithRoot" null null))
      (`GameplayStatics.PlaySoundAtLocation` "/Game/StudentWork/Audio_Project_Files/ProjectileMETASOUND.ProjectileMETASOUND" (`self.K2_GetActorLocation`) (struct) 1.0 1.0 0.0 "/Game/StudentWork/Audio_Project_Files/explosion_SA.explosion_SA" "/Game/StudentWork/Audio_Project_Files/ProjectileExplosion_SC.ProjectileExplosion_SC" _returnvalue_2 null))))

(fn `UserConstructionScript`
  (`parent.UserConstructionScript`))