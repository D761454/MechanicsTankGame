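; Assault enemy variant that carries a key, spawning a BP_PassKey at its location when killed.
; Incoming damage lowers CurrentHealth, and at zero it deals radial damage around its mesh, plays a world camera shake and spawns a Niagara explosion.
; It also calls DestroyEvent on death, and construction defers to the parent class.
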(event `self.ReceiveAnyDamage`
  (params (Damage :type "Float (single-precision)") (DamageType :type "DamageType Object Reference") (InstigatedBy :type "Controller Object Reference") (DamageCauser :type "Actor Object Reference"))
  (bind _returnvalue (`self.K2_GetActorLocation`))
  ;[1 0.9435 0] Damage Event
  (set `self.CurrentHealth` (- (`self.CurrentHealth`) Damage))
  (if (<= (`self.CurrentHealth`) 0.0)
    ;[1 1 1] Radial Dmg and Explosion
    (`GameplayStatics.ApplyRadialDamage` :`BaseDamage` 5.0 :`Origin` (`SceneComponent.K2_GetComponentLocation` (`self.StaticMesh`)) :`DamageRadius` 150.0 :`DamageTypeClass` "/Script/Engine.DamageType" :`DamageCauser` self :`InstigatedByController` null :`bDoFullDamage` true)
    (`GameplayStatics.PlayWorldCameraShake` "/Game/StudentWork/CamShakes/CS_Death.CS_Death_C" _returnvalue 0.1 3000.0 0.1)
    (`self.DestroyEvent`)
    (`NiagaraFunctionLibrary.SpawnSystemAtLocation` "/Game/StudentWork/Particles/Death/NS_Explosion.NS_Explosion" _returnvalue)
    (`|SpawnActorFromClass` "/Game/StudentWork/LevelDynamics/BP_PassKey.BP_PassKey_C" (`self.GetTransform`) "Undefined" "MultiplyWithRoot" null null)))

(event `CustomEvent`
  ;[1 0.9435 0] Damage Event
  (`self.K2_DestroyActor`))

(fn `UserConstructionScript`
  (`parent.UserConstructionScript`))