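; BP_Enemy_Assault_Elite is an elite assault enemy Blueprint that fires projectiles in limited bursts.
; Each Attack call outside cooldown spawns an elite assault projectile at the FireArrow transform with an attenuated firing sound, then decrements Bursts.
; When Bursts runs out, a cooldown flag blocks attacks until a one-shot timer clears it and refills the count.
; The construction script only runs the parent's.
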(event `Reset Cooldown`
  (set `self.Cooldown` false)
  (set `self.Bursts` 4))

(event `self.Attack`
  (bind _firearrow (`self.FireArrow`))
  ;[1 1 1] Attack
  (if (not (`self.Cooldown`))
    (bind _returnvalue (`|SpawnActorFromClass` "/Game/StudentWork/Enemy/Assault/BP_Assault_Projectile_Elite.BP_Assault_Projectile_Elite_C" (`KismetMathLibrary.MakeTransform` (`SceneComponent.K2_GetComponentLocation` _firearrow) (`SceneComponent.K2_GetComponentRotation` _firearrow)) "Undefined" "MultiplyWithRoot" null null))
    (`GameplayStatics.PlaySoundAtLocation` "/Game/StudentWork/Audio_Project_Files/ProjectileMETASOUND.ProjectileMETASOUND" (`self.K2_GetActorLocation`) (struct) 1.0 1.0 0.0 "/Game/StudentWork/Audio_Project_Files/explosion_SA.explosion_SA" "/Game/StudentWork/Audio_Project_Files/ProjectileExplosion_SC.ProjectileExplosion_SC" _returnvalue null)
    (bind _result (`/Engine/EditorBlueprintResources/StandardMacros.DecrementInt` (`self.Bursts`))
      (:`  `
        (if (<= _result 0)
          (set `self.Cooldown` true)
          (`KismetSystemLibrary.K2_SetTimerDelegate` (delegate `Reset Cooldown`) (`self.Cooldown Speed`)))))))

(fn `UserConstructionScript`
  (`parent.UserConstructionScript`))