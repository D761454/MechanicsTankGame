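; Key-holder boss variant of the assault enemy that overrides its parent's movement and attack events.
; Move sends it to a random reachable point near its target.
; Attack rolls randomly between a tank projectile, a homing missile locked to the target's capsule, or doing nothing.
; High rolls call radial damage instead when the target overlaps the AOE zone, though only the full-damage flag is set.
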(event `self.Move`
  ;[1 1 1] Movement
  (`|AIMoveTo` self (`NavigationSystemV1.K2_GetRandomReachablePointInRadius` (`self.K2_GetActorLocation` (`self.MyTarget`)) 600.0 null null) null 30.0))

(event `self.Attack`
  (bind _mytarget (`self.MyTarget`))
  (bind _firearrow (`self.FireArrow`))
  (bind _returnvalue (`SceneComponent.K2_GetComponentLocation` _firearrow))
  (bind _returnvalue_2 (`SceneComponent.K2_GetComponentRotation` _firearrow))
  (bind _output_get (set `self.Rand` (`KismetMathLibrary.RandomIntegerInRange` 0 10)))
  (if (> _output_get 5)
    (if (`PrimitiveComponent.IsOverlappingActor` (`self.AOEZone`) (`self.MyTarget`))
      (if (> _output_get 8)
        (`GameplayStatics.ApplyRadialDamage` :`DamageCauser` null :`InstigatedByController` null :`bDoFullDamage` true)
        (else
          ;[1 1 1] TANK
          (bind _returnvalue_3 (`|SpawnActorFromClass` "/Game/StudentWork/Enemy/Tank/BP_Tank_Projectile.BP_Tank_Projectile_C" (`KismetMathLibrary.MakeTransform` _returnvalue _returnvalue_2) "Undefined" "MultiplyWithRoot" null null :!label _label))
          (`GameplayStatics.PlaySoundAtLocation` "/Game/StudentWork/Audio_Project_Files/ProjectileMETASOUND.ProjectileMETASOUND" (`self.K2_GetActorLocation`) (struct) 1.0 1.0 0.0 "/Game/StudentWork/Audio_Project_Files/explosion_SA.explosion_SA" "/Game/StudentWork/Audio_Project_Files/ProjectileExplosion_SC.ProjectileExplosion_SC" _returnvalue_3 null)
          (`NiagaraFunctionLibrary.SpawnSystemAtLocation` "/Game/StudentWork/Particles/ProjHit/NS_Fire_B.NS_Fire_B" _returnvalue _returnvalue_2)))
      (else
        (goto _label)))
    (elif (> _output_get 2)
      (`/Engine/EditorBlueprintResources/StandardMacros.IsValid` _mytarget
        (:`Is Valid`
          ;[1 1 1] MISSILE
          (bind _returnvalue_4 (`|SpawnActorFromClass` "/Game/StudentWork/Enemy/BP_Enemy_Homing_Projectile.BP_Enemy_Homing_Projectile_C" (`KismetMathLibrary.MakeTransform` _returnvalue (`KismetMathLibrary.FindLookAtRotation` _returnvalue (`self.K2_GetActorLocation` _mytarget))) "Undefined" "MultiplyWithRoot" null null))
          (`GameplayStatics.PlaySoundAtLocation` "/Game/StudentWork/Audio_Project_Files/ProjectileMETASOUND.ProjectileMETASOUND" (`self.K2_GetActorLocation`) (struct) 1.0 1.0 0.0 "/Game/StudentWork/Audio_Project_Files/explosion_SA.explosion_SA" "/Game/StudentWork/Audio_Project_Files/ProjectileExplosion_SC.ProjectileExplosion_SC" _returnvalue_4 null)
          (`NiagaraFunctionLibrary.SpawnSystemAtLocation` "/Game/StudentWork/Particles/ProjHit/NS_Fire_R.NS_Fire_R" _returnvalue _returnvalue_2)
          (set `ProjectileMovementComponent.HomingTargetComponent` (`Character.CapsuleComponent` _mytarget) (`/Game/StudentWork/Enemy/BP_Enemy_Homing_Projectile.ProjectileMovement` _returnvalue_4)))))))

(fn `UserConstructionScript`
  (`parent.UserConstructionScript`))