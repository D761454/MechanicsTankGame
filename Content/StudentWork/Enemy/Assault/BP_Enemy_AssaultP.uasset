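; BP_Enemy_AssaultP is an assault enemy Blueprint that chases its target and fires projectiles.
; Its Move event sends the pawn toward a valid MyTarget with AI MoveTo.
; Its Attack event spawns an assault projectile at the FireArrow component, randomizing direction within a cone sized by Accuracy for spread.
; Each shot also plays an attenuated, concurrency-limited MetaSound and a Niagara muzzle effect.
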(event `self.Move`
  (bind _mytarget (`self.MyTarget`))
  ;[1 1 1] Movement
  (`/Engine/EditorBlueprintResources/StandardMacros.IsValid` _mytarget
    (:`Is Valid`
      (`|AIMoveTo` self (0.0 0.0 0.0) _mytarget 30.0))))

(event `self.Attack`
  (bind _firearrow (`self.FireArrow`))
  (bind _returnvalue (`SceneComponent.K2_GetComponentLocation` _firearrow))
  (bind _returnvalue_2 (`SceneComponent.K2_GetComponentRotation` _firearrow))
  ;[1 1 1] Attack
  (bind _returnvalue_3 (`|SpawnActorFromClass` "/Game/StudentWork/Enemy/Assault/BP_Assault_Projectile.BP_Assault_Projectile_C" (`KismetMathLibrary.MakeTransform` _returnvalue (`KismetMathLibrary.Conv_VectorToRotator` (`KismetMathLibrary.RandomUnitVectorInConeInDegrees` (`KismetMathLibrary.Conv_RotatorToVector` _returnvalue_2) (`self.Accuracy`)))) "Undefined" "MultiplyWithRoot" null null))
  (`GameplayStatics.PlaySoundAtLocation` "/Game/StudentWork/Audio_Project_Files/ProjectileMETASOUND.ProjectileMETASOUND" (`self.K2_GetActorLocation`) (struct) 1.0 1.0 0.0 "/Game/StudentWork/Audio_Project_Files/explosion_SA.explosion_SA" "/Game/StudentWork/Audio_Project_Files/ProjectileExplosion_SC.ProjectileExplosion_SC" _returnvalue_3 null)
  (`NiagaraFunctionLibrary.SpawnSystemAtLocation` "/Game/StudentWork/Particles/ProjHit/NS_Fire_R.NS_Fire_R" _returnvalue _returnvalue_2))

(fn `UserConstructionScript`
  (`parent.UserConstructionScript`))