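; BP_Enemy_Security_Rocket is a security enemy variant that attacks its target by firing homing rockets.
; Its Attack event spawns a homing projectile at the FireArrow, rotated to face the current target.
; The projectile's movement component then takes the target's capsule as its homing target, with validity checks before spawning and before assigning it.
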(event `self.Attack`
  (bind _mytarget (`self.MyTarget`))
  (bind _mytarget_2 (`self.MyTarget`))
  (bind _returnvalue (`SceneComponent.K2_GetComponentLocation` (`self.FireArrow`)))
  ;[1 0 0] Attack Player
  (`/Engine/EditorBlueprintResources/StandardMacros.IsValid` _mytarget
    (:`Is Valid`
      (bind _returnvalue_2 (`|SpawnActorFromClass` "/Game/StudentWork/Enemy/BP_Enemy_Homing_Projectile.BP_Enemy_Homing_Projectile_C" (`KismetMathLibrary.MakeTransform` _returnvalue (`KismetMathLibrary.FindLookAtRotation` _returnvalue (`self.K2_GetActorLocation` _mytarget))) "Undefined" "MultiplyWithRoot" null null))
      (`/Engine/EditorBlueprintResources/StandardMacros.IsValid` _mytarget_2
        (:`Is Valid`
          (set `ProjectileMovementComponent.HomingTargetComponent` (`Character.CapsuleComponent` _mytarget_2) (`/Game/StudentWork/Enemy/BP_Enemy_Homing_Projectile.ProjectileMovement` _returnvalue_2)))))))

(fn `UserConstructionScript`
  (`parent.UserConstructionScript`))