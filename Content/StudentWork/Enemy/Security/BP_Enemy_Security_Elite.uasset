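; BP_Enemy_Security_Elite is an elite security enemy that wanders and fires projectiles at its target.
; The Move event sends it by AIMoveTo to a random reachable point within a radius of its current location.
; The Attack event checks that MyTarget is valid, then spawns BP_Security_Projectile_Elite at FireArrow, rotated toward the target's location.
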(event `self.Move`
  ;[1 1 1] Movement
  (`|AIMoveTo` self (`NavigationSystemV1.K2_GetRandomReachablePointInRadius` (`self.K2_GetActorLocation`) 600.0 null null) null 10.0))

(event `self.Attack`
  (bind _mytarget (`self.MyTarget`))
  (bind _returnvalue (`SceneComponent.K2_GetComponentLocation` (`self.FireArrow`)))
  ;[1 0 0] Attack Player
  (`/Engine/EditorBlueprintResources/StandardMacros.IsValid` _mytarget
    (:`Is Valid`
      (`|SpawnActorFromClass` "/Game/StudentWork/Enemy/Security/BP_Security_Projectile_Elite.BP_Security_Projectile_Elite_C" (`KismetMathLibrary.MakeTransform` _returnvalue (`KismetMathLibrary.FindLookAtRotation` _returnvalue (`self.K2_GetActorLocation` _mytarget))) "Undefined" "MultiplyWithRoot" null null))))

(fn `UserConstructionScript`
  (`parent.UserConstructionScript`))