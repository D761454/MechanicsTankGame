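; BP_Target_Large is an explosive barrel target that flashes and then explodes when it takes any damage.
; The construction script gives the barrel a dynamic material, whose FlashLevel a timeline drives after the first hit, gated by DoOnce.
; When the flash finishes, it applies full radial damage around the barrel, shakes nearby cameras, destroys itself, and spawns a Niagara explosion with attenuated sound.
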(event `DestroyEvent`
  ;[1 1 1] Flash Event
  (`self.K2_DestroyActor`))

(event `self.ReceiveAnyDamage`
  (params (Damage :type "Float (single-precision)") (DamageType :type "DamageType Object Reference") (InstigatedBy :type "Controller Object Reference") (DamageCauser :type "Actor Object Reference"))
  (bind _returnvalue (`self.K2_GetActorLocation`))
  ;[1 1 1] Flash Event
  (`/Engine/EditorBlueprintResources/StandardMacros.DoOnce` false
    (:`Completed`
      (bind (_direction _flash) (`Timeline|Flash` :!via `PlayFromStart`)
        (:`Update`
          (`MaterialInstanceDynamic.SetScalarParameterValue` (`self.Flash Material`) "FlashLevel" _flash))
        (:`Finished`
          ;[1 1 1] Radial Dmg and Explosion
          (`GameplayStatics.ApplyRadialDamage` :`BaseDamage` 10.0 :`Origin` (`SceneComponent.K2_GetComponentLocation` (`self.SM_Barrel`)) :`DamageRadius` 500.0 :`DamageTypeClass` "/Script/Engine.DamageType" :`DamageCauser` self :`InstigatedByController` null :`bDoFullDamage` true)
          (`GameplayStatics.PlayWorldCameraShake` "/Game/StudentWork/CamShakes/CS_Explosion_Large.CS_Explosion_Large_C" (`self.K2_GetActorLocation`) 0.1 3000.0 0.1)
          (`self.DestroyEvent`)
          (`NiagaraFunctionLibrary.SpawnSystemAtLocation` "/Game/StudentWork/Particles/Death/NS_Explosion.NS_Explosion" _returnvalue)
          (`GameplayStatics.PlaySoundAtLocation` "/Game/StudentWork/Audio_Project_Files/ExplosionMETASOUND.ExplosionMETASOUND" _returnvalue (struct) 1.0 1.0 0.0 "/Game/StudentWork/Audio_Project_Files/explosion_SA.explosion_SA" "/Game/StudentWork/Audio_Project_Files/ProjectileExplosion_SC.ProjectileExplosion_SC" null null))))))

(fn `UserConstructionScript`
  (bind _returnvalue (`PrimitiveComponent.CreateDynamicMaterialInstance` (`self.SM_Barrel`) 0 "/Game/StudentWork/Materials/FX/M_Target_Death_2.M_Target_Death_2" "None"))
  (set `self.Flash Material` _returnvalue))