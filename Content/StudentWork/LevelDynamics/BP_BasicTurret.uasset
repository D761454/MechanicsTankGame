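; BP_BasicTurret is an enemy turret actor that fires projectiles on a fixed interval and explodes when destroyed.
; A looping timer set on BeginPlay spawns BP_EnemyProjectile at its Arrow component's location and rotation.
; AnyDamage reduces CurrentHealth, and at zero or below the turret deals radial damage, plays a death camera shake, destroys itself and spawns a Niagara explosion.
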(event `self.ReceiveBeginPlay`
  ;[1 1 1] Firing
  (bind _returnvalue (`KismetSystemLibrary.K2_SetTimerDelegate` (delegate `Fire Projectile`) 1.25 true))
  (set `self.Fire Timer` _returnvalue))

(event `Fire Projectile`
  (bind _arrow (`self.Arrow`))
  ;[1 1 1] Firing
  (`|SpawnActorFromClass` "/Game/StudentWork/Enemy/BP_EnemyProjectile.BP_EnemyProjectile_C" (`KismetMathLibrary.MakeTransform` (`SceneComponent.K2_GetComponentLocation` _arrow) (`SceneComponent.K2_GetComponentRotation` _arrow)) "Undefined" "MultiplyWithRoot" null null))

(event `self.ReceiveAnyDamage`
  (params (Damage :type "Float (single-precision)") (DamageType :type "DamageType Object Reference") (InstigatedBy :type "Controller Object Reference") (DamageCauser :type "Actor Object Reference"))
  (bind _returnvalue (`self.K2_GetActorLocation`))
  ;[1 1 1] Damage Event
  (set `self.CurrentHealth` (- (`self.CurrentHealth`) Damage))
  (if (<= (`self.CurrentHealth`) 0.0)
    ;[1 1 1] Death and Radial Dmg
    (`GameplayStatics.ApplyRadialDamage` :`BaseDamage` 10.0 :`Origin` (`SceneComponent.K2_GetComponentLocation` (`self.StaticMesh`)) :`DamageRadius` 200.0 :`DamageTypeClass` "/Script/Engine.DamageType" :`DamageCauser` self :`InstigatedByController` null :`bDoFullDamage` true)
    (`GameplayStatics.PlayWorldCameraShake` "/Game/StudentWork/CamShakes/CS_Death.CS_Death_C" _returnvalue 0.1 3000.0 0.1)
    (`self.DestroyEvent`)
    (`NiagaraFunctionLibrary.SpawnSystemAtLocation` "/Game/StudentWork/Particles/Death/NS_Explosion.NS_Explosion" _returnvalue)))

(event `DestroyEvent`
  ;[1 1 1] Damage Event
  (`self.K2_DestroyActor`))

(fn `UserConstructionScript`)