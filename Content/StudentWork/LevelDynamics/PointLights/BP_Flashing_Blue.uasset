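; BP_Flashing_Blue is a point light Blueprint that pulses its intensity up and down continuously during play.
; BeginPlay calls CustomTick, which starts a fast looping timer in place of Tick.
; Each timer step adds or subtracts TimeScale from the PointLight intensity, and the Change flag reverses direction at fixed upper and zero bounds, giving a linear ping-pong fade.
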(event `CustomTick`
  (`KismetSystemLibrary.K2_SetTimerDelegate` (delegate `Millisec`) 0.1 true))

(event `Millisec`
  (bind _pointlight (`self.PointLight`))
  (bind _timescale (`self.TimeScale`))
  (bind _intensity (`LightComponentBase.Intensity` (`self.PointLight`)))
  (if (`self.Change`)
    (`LightComponent.SetIntensity` _pointlight (+ _intensity _timescale))
    (if (>= _intensity 1000.0)
      (set `self.Change` false))
    (else
      (`LightComponent.SetIntensity` _pointlight (- _intensity _timescale))
      (if (<= _intensity 0.0)
        (set `self.Change` true)))))

(event `self.ReceiveBeginPlay`
  (`self.CustomTick`))

(fn `UserConstructionScript`)