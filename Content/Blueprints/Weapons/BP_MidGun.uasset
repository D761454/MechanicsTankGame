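; BP_MidGun is a tank weapon that fires a BP_Projectile when triggered.
; The projectile spawns at the location and rotation of the owning tank's DirectionArrow, and each shot plays the CS_RegFire camera shake on the first player's camera.
; A Cooldown flag, cleared by a short one-shot timer, limits the fire rate by ignoring triggers until it resets.
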(event `self.Triggered`
  (bind _directionarrow (`/Game/Blueprints/BP_PlayerCharacter.DirectionArrow` (`self.MyTank`)))
  (if (not (`self.Cooldown`))
    (`|SpawnActorFromClass` "/Game/StudentWork/Player/Projectiles/BP_Projectile.BP_Projectile_C" (`KismetMathLibrary.MakeTransform` (`SceneComponent.K2_GetComponentLocation` _directionarrow) (`SceneComponent.K2_GetComponentRotation` _directionarrow)) "Undefined" "MultiplyWithRoot" null null)
    (`PlayerCameraManager.StartCameraShake` :`self` (`GameplayStatics.GetPlayerCameraManager` 0) :`ShakeClass` "/Game/StudentWork/CamShakes/CS_RegFire.CS_RegFire_C")
    (set `self.Cooldown` true)
    (`KismetSystemLibrary.K2_SetTimerDelegate` (delegate `End Cooldown`) 0.5)))

(event `End Cooldown`
  (set `self.Cooldown` false))

(fn `UserConstructionScript`
  (`parent.UserConstructionScript`))